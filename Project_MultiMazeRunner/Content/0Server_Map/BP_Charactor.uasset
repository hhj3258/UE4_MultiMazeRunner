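; BP_Charactor is an enemy actor that hurts a KallariPlayerCharacter on overlap and opens a wall when destroyed.
; Incoming damage lowers EnemyHealth through a DoOnce reset after a short delay, throttling hits until health runs out and the actor destroys itself.
; Its Destroyed event calls OpenWall on OpenSet, and SetMode stores a mode that shows or hides the Reds component.
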(event Collision|EventActorBeginOverlap
  (params (OtherActor :type Actor%20Object%20Reference))
  ;[1 1 1] 플레이어에게 대미지
  (bind _askallari_player_character (Utilities|Casting|CastToKallariPlayerCharacter OtherActor))
  (Game|Damage|ApplyDamage _askallari_player_character 0.09 0 0))

(event Game|Damage|EventAnyDamage
  (params (Damage :type Float%20%28single-precision%29) (DamageType :type Damage%20Type%20Object%20Reference) (InstigatedBy :type Controller%20Object%20Reference) (DamageCauser :type Actor%20Object%20Reference))
  ;[1 1 1] 적을 죽이면 삭제
  (Development|PrintString "EnAttacked")
  (Utilities|FlowControl|DoOnce false :!label _label
    (:Completed
      (bind _output_get (Variables|Default|SetEnemyHealth (- (Variables|Default|GetEnemyHealth) Damage)))
      (if (<= _output_get 0.0)
        (Development|PrintString "Quit")
        (Actor|DestroyActor)
        (else
          (Development|PrintString (Utilities|String|ToString(Float) (Variables|Default|GetEnemyHealth)))
          (Utilities|FlowControl|Delay 0.3)
          (goto _label Reset))))))

(event EventDestroyed
  ;[1 1 1] 삭제되면 문 열림
  (Default|OpenWall (Variables|Default|GetOpenSet)))

(fn ConstructionScript)

(fn SetMode
  (params (mode :type Integer))
  (bind _output_get (Variables|Default|Setmode mode))
  (switch int _output_get
    (:0
      (Rendering|SetVisibility (Variables|Default|GetReds) false false))
    (:1
      (Rendering|SetVisibility (Variables|Default|GetReds) true false))))